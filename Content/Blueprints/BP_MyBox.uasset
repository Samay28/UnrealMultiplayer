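; BP_MyBox is a debug-style box Blueprint that displays its network authority and a replicated variable as text.
; On BeginPlay, it sets AuthorityText according to whether the instance has authority.
; Every Tick, it writes ReplicatedValue into VarText with a label, though nothing in these graphs changes that value.
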(event EventBeginPlay
  (if (Ability|HasAuthority)
    (Rendering|Components|TextRender|SetText (Variables|Default|GetAuthorityText) (Utilities|Text|ToText(String) (Utilities|String|MakeLiteralString "has Authority")))
    (else
      (Rendering|Components|TextRender|SetText (Variables|Default|GetAuthorityText) (Utilities|Text|ToText(String) (Utilities|String|MakeLiteralString "no Authority"))))))

(event EventTick
  (params (DeltaSeconds :type Float%20%28single-precision%29))
  (Rendering|Components|TextRender|SetText (Variables|Default|GetVarText) (Utilities|Text|ToText(String) (Utilities|String|Append (Utilities|String|MakeLiteralString "Replicated Var :") (Utilities|String|ToString(Float) (Variables|Default|GetReplicatedValue))))))

(fn ConstructionScript)